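; MyAvatar is a player-controlled avatar with axis-driven look and movement that also operates lights through debug-style key presses.
; B toggles its Light between dim and bright using the Intensity boolean.
; At BeginPlay it caches the Tutorial_BP actor as TutorialLight, whose TutBPLight is controlled by FlipFlops: O alternates between two colors and P between bright and dim.
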(event `InputAxis|mouseUp`
  (params (AxisValue :type "Float (single-precision)"))
  (`self.AddControllerPitchInput` AxisValue))

(event `InputAxis|MouseRight`
  (params (AxisValue :type "Float (single-precision)"))
  (`self.AddControllerYawInput` AxisValue))

(event `InputAxis|Right`
  (params (AxisValue :type "Float (single-precision)"))
  (`self.AddMovementInput` (`self.GetActorRightVector`) AxisValue))

(event `InputAxis|Forward`
  (params (AxisValue :type "Float (single-precision)"))
  (`self.AddMovementInput` (`self.GetActorForwardVector`) AxisValue))

(event `Key|B`
  (params (Key :type "Key Structure"))
  (bind _light (`self.Light`))
  (:`Pressed`
    (if (`self.Intensity`)
      (`LightComponent.SetIntensity` _light 1.0)
      (set `self.Intensity` false)
      (else
        (`LightComponent.SetIntensity` _light 50000.0)
        (set `self.Intensity` true)))))

(event `Key|O`
  (params (Key :type "Key Structure"))
  (bind _tutbplight (`/Game/Blueprints/Tutorial_BP.TutBPLight` (`self.Tutorial Light`)))
  (:`Pressed`
    (`/Engine/EditorBlueprintResources/StandardMacros.FlipFlop`
      (:`A`
        (`LightComponent.SetLightColor` _tutbplight (struct :`G` 0.540772 :`B` 0.572917 :`A` 1.0) true))
      (:`B`
        (`LightComponent.SetLightColor` _tutbplight (struct :`R` 1.0 :`G` 0.140625 :`B` 0.961442 :`A` 1.0) true)))))

(event `self.ReceiveBeginPlay`
  (bind _returnvalue (`GameplayStatics.GetActorOfClass` "/Game/Blueprints/Tutorial_BP.Tutorial_BP_C"))
  (set `self.Tutorial Light` _returnvalue))

(event `Key|P`
  (params (Key :type "Key Structure"))
  (bind _tutbplight (`/Game/Blueprints/Tutorial_BP.TutBPLight` (`self.Tutorial Light`)))
  (:`Pressed`
    (`/Engine/EditorBlueprintResources/StandardMacros.FlipFlop`
      (:`A`
        (`LightComponent.SetIntensity` _tutbplight 50000.0))
      (:`B`
        (`LightComponent.SetIntensity` _tutbplight 1.0)))))

(event `self.ReceiveActorBeginOverlap`
  (params (OtherActor :type "Actor Object Reference")))

(fn `UserConstructionScript`)