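; Tutorial Blueprint whose light, TutBPLight, alternates between very bright and nearly off.
; BeginPlay starts it bright, then Tick branches on the Intensity boolean through Delay nodes to flip the state about every ten seconds.
; The IntensityControl input axis also adds its value to the light's current intensity.
; A TimeElapsed addition is left unconnected and never runs.
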(event `self.ReceiveBeginPlay`
  (`LightComponent.SetIntensity` (`self.TutBPLight`) 50000.0)
  (set `self.Intensity` true))

(event `self.ReceiveTick`
  (params (DeltaSeconds :type "Float (single-precision)"))
  (if (`self.Intensity`)
    (`KismetSystemLibrary.Delay` 10.0)
    (`LightComponent.SetIntensity` (`self.TutBPLight`) 1.0)
    (set `self.Intensity` false)
    (else
      (`KismetSystemLibrary.Delay` 10.0)
      (`LightComponent.SetIntensity` (`self.TutBPLight`) 50000.0)
      (set `self.Intensity` true))))

(event `InputAxis|IntensityControl`
  (params (AxisValue :type "Float (single-precision)"))
  (`LightComponent.SetIntensity` (`self.TutBPLight`) (+ AxisValue (`LightComponentBase.Intensity` (`self.TutBPLight`)))))

(fn `UserConstructionScript`)